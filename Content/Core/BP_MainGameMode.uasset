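; BP_MainGameMode is the main game mode, which puts the main display widget on screen when play begins.
; BeginPlay creates WBP_MainDisplay for the first player controller, passes it the quest manager and adds it to the viewport.
; The quest manager comes through a deprecated wrapper around GetQuestManager, whose older spawn-if-missing logic for BP_QuestManager remains but never runs.
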(event EventBeginPlay
  (bind _returnvalue (UserInterface|CreateWidget "/Game/UI/WBP_MainDisplay.WBP_MainDisplay_C" (Game|GetPlayerController 0) (CallFunction|DEPREACTEDGetQuestManager)))
  (UserInterface|Viewport|AddtoViewport _returnvalue 0))

(event EventTick
  (params (DeltaSeconds :type Float%20%28single-precision%29)))

(fn ConstructionScript)

(fn DEPREACTEDGetQuestManager
  (return (Class|MainGameMode|GetQuestManager)))